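; BP_Tunnel is a tunnel segment with a spinning holed wall that the player must pass through to score.
; RandomizeWall picks one of four hole meshes and a random roll, and Tick keeps the wall rotating.
; Player overlap with TriggerZone spawns the next tunnel, destroys this one and raises score.
; Wall hits cost health and score, recolor tunnel materials by health band, and show restart once health drops below zero.
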(event OnComponentBeginOverlap(TriggerZone)
  (params (OverlappedComponent :type Primitive%20Component%20Object%20Reference) (OtherActor :type Actor%20Object%20Reference) (OtherComp :type Primitive%20Component%20Object%20Reference) (OtherBodyIndex :type Integer) (bFromSweep :type Boolean) (SweepResult :type Hit%20Result%20Structure%20%28by%20ref%29))
  (Utilities|FlowControl|Sequence
    (:then_0
      (Utilities|Casting|CastToBP_Player OtherActor)
      (Default|SpawnTunnelatSpawnPoint (Variables|Default|GetTunnelSpawner))
      (Actor|DestroyActor))
    (:then_1
      ;[1 1 1] Increase Score by 1 on successful passing and update the widget
      (bind (_bp_player _score) (CallFunction|UpdateScorePlayer OtherActor 1))
      (Default|UpdateScore (Variables|/Game/InfiniteMatrix/Blueprints/BP_Player.BP_Player_C|GetScoreWidget _bp_player) _score))))

(event OnComponentBeginOverlap(WallMesh)
  (params (OverlappedComponent :type Primitive%20Component%20Object%20Reference) (OtherActor :type Actor%20Object%20Reference) (OtherComp :type Primitive%20Component%20Object%20Reference) (OtherBodyIndex :type Integer) (bFromSweep :type Boolean) (SweepResult :type Hit%20Result%20Structure%20%28by%20ref%29))
  (Utilities|FlowControl|Sequence
    (:then_0
      (CallFunction|UpdateHealth OtherActor))
    (:then_1
      ;[1 1 1] Reduce score by 1 on Wall collision - don't update the widget
      (CallFunction|UpdateScorePlayer OtherActor -1))))

(event EventBeginPlay)

(event EventTick
  (params (DeltaSeconds :type Float%20%28single-precision%29))
  (Transformation|AddLocalRotation (Variables|Default|GetWall%20Mesh) (Math|Rotator|MakeRotator (* DeltaSeconds (Variables|Default|GetRotateSpeed)) 0.0 0.0) false false))

(fn ConstructionScript)

(fn RandomizeWall
  (Components|StaticMesh|SetStaticMesh (Variables|Default|GetWall%20Mesh) (Utilities|Select :Index (Math|Random|RandomIntegerinRange 0 3) :Option%200 "/Game/InfiniteMatrix/Meshes/SM_Hole_01.SM_Hole_01" :Option%201 "/Game/InfiniteMatrix/Meshes/SM_Hole_02.SM_Hole_02" :Option%202 "/Game/InfiniteMatrix/Meshes/SM_Hole_03.SM_Hole_03" :Option%203 "/Game/InfiniteMatrix/Meshes/SM_Hole_04.SM_Hole_04"))
  (Transformation|AddLocalRotation (Variables|Default|GetWall%20Mesh) (Math|Rotator|MakeRotator (Math|Random|RandomFloatinRange 0.0 3.6e+02) 0.0 0.0) false false))

(fn ChangeStaticMeshColor
  (params (Health :type Float%20%28double-precision%29))
  (bind _staticmeshcomponent (Variables|Debug|GetStaticMeshComponent))
  (Development|PrintString (Utilities|String|ToString(Float) Health))
  (if (Math|Float|InRange(Float) Health 7e+01 1e+02)
    (Rendering|Material|SetVectorParameterValueonMaterials _staticmeshcomponent "BackgroundColor" "10.000000,10.000000,10.000000")
    (Rendering|Material|SetVectorParameterValueonMaterials _staticmeshcomponent "TextColor" "0, 0, 0")
    (elif (Math|Float|InRange(Float) Health 3e+01 69.0)
      (Rendering|Material|SetVectorParameterValueonMaterials _staticmeshcomponent "BackgroundColor" "0.380000,0.120000,0.009000")
      (Rendering|Material|SetVectorParameterValueonMaterials _staticmeshcomponent "TextColor" "1.000000,0.500000,0.100000")
      (elif (Math|Float|InRange(Float) Health 0.0 29.0)
        (Rendering|Material|SetVectorParameterValueonMaterials _staticmeshcomponent "BackgroundColor" "0.300000,0.007000,0.030000")
        (Rendering|Material|SetVectorParameterValueonMaterials _staticmeshcomponent "TextColor" "1.000000,0.200000,0.200000")))))

(fn UpdateHealth
  (params (Actor :type Actor%20Object%20Reference))
  ;[1 1 1] Update Health - Reduces 25 points on every overlap with the wall
  (bind _asbp_player (Utilities|Casting|CastToBP_Player Actor))
  (bind _output_get (Variables|/Game/InfiniteMatrix/Blueprints/BP_Player.BP_Player_C|SetCurrHealth _asbp_player (- (Variables|/Game/InfiniteMatrix/Blueprints/BP_Player.BP_Player_C|GetCurrHealth _asbp_player) 25.0)))
  (Default|UpdateHealthBar (Variables|/Game/InfiniteMatrix/Blueprints/BP_Player.BP_Player_C|GetHealthWidget _asbp_player) _output_get (Variables|/Game/InfiniteMatrix/Blueprints/BP_Player.BP_Player_C|GetMaxHealth _asbp_player))
  (CallFunction|ChangeStaticMeshColor _output_get)
  (bind _output_get_2 (Variables|/Game/InfiniteMatrix/Blueprints/BP_Player.BP_Player_C|SetisDead _asbp_player (< _output_get 0.0)))
  (if _output_get_2
    (Default|DisplayRestart _asbp_player)))

(fn UpdateScorePlayer
  (params (Actor :type Actor%20Object%20Reference) (Value :type Integer))
  (bind _asbp_player (Utilities|Casting|CastToBP_Player Actor))
  (bind _output_get (Variables|/Game/InfiniteMatrix/Blueprints/BP_Player.BP_Player_C|SetScore _asbp_player (+ (Variables|/Game/InfiniteMatrix/Blueprints/BP_Player.BP_Player_C|GetScore _asbp_player) Value)))
  (return _asbp_player _output_get))